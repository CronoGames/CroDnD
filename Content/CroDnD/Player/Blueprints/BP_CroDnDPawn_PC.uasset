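; BP_CroDnDPawn_PC is a player pawn for CroDnD that handles Enhanced Input movement.
; On BeginPlay it caches the BP_CroDnDPlayerController and adds the IMC_CroDnD mapping context.
; IA_Move feeds movement input along directions derived from control rotation, with forward movement using yaw only.
; IA_Look does nothing, as its controller yaw and pitch nodes are left disconnected.
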(event Input|EnhancedActionEvents|EnhancedInputActionIA_Move
  (params (ActionValue :type Vector%202D%20Structure) (ElapsedSeconds :type Float%20%28double-precision%29) (TriggeredSeconds :type Float%20%28double-precision%29) (InputAction :type Input%20Action%20Object%20Reference :default "/Game/CroDnD/Player/Input/IA_Move.IA_Move"))
  (bind _returnvalue (Pawn|GetControlRotation :!class /Script/Engine.Pawn))
  (bind (_x _y) (Math|Vector2D|BreakVector2D ActionValue))
  (Pawn|Input|AddMovementInput (Math|Vector|GetRightVector (Math|Rotator|MakeRotator (.roll _returnvalue) 0.0 (.yaw _returnvalue))) _x false)
  (Pawn|Input|AddMovementInput (Math|Vector|GetForwardVector (Math|Rotator|MakeRotator 0.0 0.0 (.yaw (Pawn|GetControlRotation :!class /Script/Engine.Pawn)))) _y false))

(event Input|EnhancedActionEvents|EnhancedInputActionIA_Look
  (params (ActionValue :type Vector%202D%20Structure) (ElapsedSeconds :type Float%20%28double-precision%29) (TriggeredSeconds :type Float%20%28double-precision%29) (InputAction :type Input%20Action%20Object%20Reference :default "/Game/CroDnD/Player/Input/IA_Look.IA_Look")))

(event EventBeginPlay
  (bind _asbp_cro_dn_dplayer_controller (Utilities|Casting|CastToBP_CroDnDPlayerController (Pawn|GetController)))
  (Variables|Default|SetPlayerControllerRef _asbp_cro_dn_dplayer_controller)
  (Utilities|IsValid (PlayerController|LocalPlayerSubsystems|GetEnhancedInputLocalPlayerSubsystem _asbp_cro_dn_dplayer_controller)
    (:Is%20Valid
      (Input|AddMappingContext (PlayerController|LocalPlayerSubsystems|GetEnhancedInputLocalPlayerSubsystem _asbp_cro_dn_dplayer_controller) "/Game/CroDnD/Player/Input/IMC_CroDnD.IMC_CroDnD" 0 "(bIgnoreAllPressedKeysUntilRelease=True,bForceImmediately=False,bNotifyUserSettings=False)"))))

(fn ConstructionScript)